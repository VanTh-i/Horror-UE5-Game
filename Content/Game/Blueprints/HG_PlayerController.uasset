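; Player controller that applies sensitivity-scaled look input and toggles the inventory menu on the OpenInventory action.
; BeginPlay creates the inventory widget collapsed in the viewport, and ToggleInventory shows or collapses it while switching input mode, cursor, look input and the player HUD crosshair.
; Opening also removes the examination widget and caches the BP_Player reference, which closing reuses before closing the menu's drop-down.
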(event `self.ReceiveBeginPlay`
  (bind _returnvalue (`|CreateWidget` "/Game/Game/Blueprints/UI/WBP_InventoryMenu.WBP_InventoryMenu_C"))
  (bind _output_get (set `self.W_InventoryMenu_Ref` _returnvalue))
  (`Widget.SetVisibility` _output_get "Collapsed")
  (`UserWidget.AddToViewport` (`self.W_InventoryMenu_Ref`) 0))

(event `InputAxis|LockUp`
  (params (AxisValue :type "Float (single-precision)"))
  (`self.AddPitchInput` (* AxisValue (`self.LookSensitivity`))))

(event `InputAxis|LockRight`
  (params (AxisValue :type "Float (single-precision)"))
  (`self.AddYawInput` (* AxisValue (`self.LookSensitivity`))))

(event `InputAction|OpenInventory`
  (params (Key :type "Key Structure"))
  (:`Pressed`
    (`self.ToggleInventory`)))

(event `ToggleInventory`
  (bind _w_inventorymenu_ref (`self.W_InventoryMenu_Ref`))
  (if (`self.IsOpenInventory?`)
    (set `self.IsOpenInventory?` false)
    (`self.ResetIgnoreLookInput`)
    (set `self.bShowMouseCursor` false)
    (`Widget.SetVisibility` _w_inventorymenu_ref "Collapsed")
    (`WidgetBlueprintLibrary.SetInputMode_GameOnly` self)
    (bind _wbp_crosshair (`/Game/Game/Blueprints/UI/WBP_HUD.WBP_Crosshair` (`/Game/Game/Blueprints/BP_Player.MainHUB_Ref` (stale _asbp_player))))
    (`Widget.SetVisibility` _wbp_crosshair "Visible")
    (`/Game/Game/Blueprints/UI/WBP_InventoryMenu.CloseDropDownMenu` (`self.W_InventoryMenu_Ref`))
    (else
      (set `self.IsOpenInventory?` true)
      (`self.SetIgnoreLookInput` true)
      (set `self.bShowMouseCursor` true)
      (`Widget.SetVisibility` _w_inventorymenu_ref "SelfHitTestInvisible")
      (`WidgetBlueprintLibrary.SetInputMode_GameAndUIEx` self (`self.W_InventoryMenu_Ref`))
      (bind _asbp_player (cast `/Game/Game/Blueprints/BP_Player` (`GameplayStatics.GetPlayerCharacter` 0)))
      (`Widget.SetVisibility` _wbp_crosshair "Hidden")
      (`Widget.RemoveFromParent` (`self.W_Examination_Ref`)))))

(fn `UserConstructionScript`)