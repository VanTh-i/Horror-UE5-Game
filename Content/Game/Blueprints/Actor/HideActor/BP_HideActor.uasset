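; BP_HideActor is an interactable hiding spot that moves the player into a hide position and back out to an exit position.
; Interact starts a looping frame-delta timer that slides the player at constant speed toward the point chosen by the player's IsHiding state.
; Collision and movement are disabled on entry and restored after exit.
; On arrival the timer clears, IsHiding flips and a finished-moving dispatcher fires.
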(event `self.ReceiveBeginPlay`
  (bind _asbp_player (cast `/Game/Game/Blueprints/BP_Player` (`GameplayStatics.GetPlayerCharacter` 0)))
  (set `self.Player_Ref` _asbp_player))

(event `/Game/Game/Blueprints/Interface/BPI_Interaction.Interact`
  (bind _player_ref (`self.Player_Ref`))
  (if (`/Game/Game/Blueprints/BP_Player.IsHiding?` (`self.Player_Ref`))
    (bind _returnvalue (`KismetSystemLibrary.K2_SetTimerDelegate` (delegate `MoveCharacter`) (`GameplayStatics.GetWorldDeltaSeconds`) true))
    (else
      (`self.SetActorEnableCollision` _player_ref false)
      (`CharacterMovementComponent.DisableMovement` (`Character.CharacterMovement` _player_ref))
      (bind _returnvalue_2 (`KismetSystemLibrary.K2_SetTimerDelegate` (delegate `MoveCharacter`) (`GameplayStatics.GetWorldDeltaSeconds`) true)))))

(event `MoveCharacter`
  (bind _player_ref (`self.Player_Ref`))
  (`self.K2_SetActorTransform` _player_ref (`KismetMathLibrary.MakeTransform` (`KismetMathLibrary.VInterpTo_Constant` (`self.K2_GetActorLocation` _player_ref) (`SceneComponent.K2_GetComponentLocation` (select `bool` (`/Game/Game/Blueprints/BP_Player.IsHiding?` (`self.Player_Ref`)) :`false` (`self.HidePosition`) :`true` (`self.ExitPositon`) :!type "SceneComponent Object Reference")) (`GameplayStatics.GetWorldDeltaSeconds`) 400.0)) false false)
  (if (== (`self.K2_GetActorLocation` (`self.Player_Ref`)) (`SceneComponent.K2_GetComponentLocation` (select `bool` (`/Game/Game/Blueprints/BP_Player.IsHiding?` (`self.Player_Ref`)) :`false` (`self.HidePosition`) :`true` (`self.ExitPositon`) :!type "SceneComponent Object Reference")) :`ErrorTolerance` 0.01)
    (`KismetSystemLibrary.K2_ClearAndInvalidateTimerHandle` (stale `/Game/Game/Blueprints/Interface/BPI_Interaction.Interact` _returnvalue_2))
    (`KismetSystemLibrary.K2_ClearAndInvalidateTimerHandle` (stale `/Game/Game/Blueprints/Interface/BPI_Interaction.Interact` _returnvalue))
    (`self.FinishedMoving`)))

(event `FinishedMoving`
  (bind _player_ref (`self.Player_Ref`))
  (bind _player_ref_2 (`self.Player_Ref`))
  (`self.FinishedMovingED`)
  (if (`/Game/Game/Blueprints/BP_Player.IsHiding?` _player_ref_2)
    (set `/Game/Game/Blueprints/BP_Player.IsHiding?` false _player_ref_2)
    (`self.SetActorEnableCollision` _player_ref true)
    (`CharacterMovementComponent.SetMovementMode` (`Character.CharacterMovement` _player_ref) "MOVE_Walking" 0)
    (else
      (set `/Game/Game/Blueprints/BP_Player.IsHiding?` true _player_ref_2))))

(fn `UserConstructionScript`)