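; Locker hide actor that adds an animated swinging door to the interaction logic inherited from its parent.
; Interact plays a timeline that swings the door mesh open, then calls the parent Interact after a short delay.
; The FinishedMovingED dispatcher, bound on BeginPlay, triggers a second timeline after a brief delay to swing the door shut.
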(event `self.ReceiveBeginPlay`
  (`parent.ReceiveBeginPlay`)
  (add `self.FinishedMovingED` (delegate `FinishedMovingED_Event`)))

(event `FinishedMovingED_Event`
  (`KismetSystemLibrary.Delay` 0.1)
  (`self.CloseDoor`))

(event `/Game/Game/Blueprints/Interface/BPI_Interaction.Interact`
  (bind (_direction _alpha) (`Timeline|OpenLockerDoorTimeline` :!via `PlayFromStart`)
    (:`Update`
      (`SceneComponent.K2_SetRelativeRotation` (`self.StaticMesh1`) (`KismetMathLibrary.MakeRotator` 0.0 0.0 (`KismetMathLibrary.Lerp` 0.0 120.0 _alpha)) false false))
    (:`Finished`
      (`KismetSystemLibrary.Delay` 0.1)
      (`parent.Interact`))))

(event `CloseDoor`
  (bind (_direction _alpha) (`Timeline|Timeline` :!via `PlayFromStart`)
    (:`Update`
      (`SceneComponent.K2_SetRelativeRotation` (`self.StaticMesh1`) (`KismetMathLibrary.MakeRotator` 0.0 0.0 (`KismetMathLibrary.Lerp` 120.0 0.0 _alpha)) false false))))

(fn `UserConstructionScript`
  (`parent.UserConstructionScript`))