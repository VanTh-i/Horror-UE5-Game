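; BP_Bandage is a usable item actor that heals the player.
; Its UseItem event checks the player's health component and, if health is below maximum, adds HealAmount and prints a debug message.
; It sets the UseItemSuccsee flag to record whether the heal was applied, so use at full health registers as a failure.
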(event `self.UseItem`
  (bind _bpc_health (`/Game/Game/Blueprints/BP_Player.BPC_Health` (`self.Player_Ref`)))
  (if (< (`/Game/Game/Blueprints/BlueprintComponent/BPC_Health.CurrentHealth` _bpc_health) (`/Game/Game/Blueprints/BlueprintComponent/BPC_Health.MaxHealth` _bpc_health))
    (`/Game/Game/Blueprints/BlueprintComponent/BPC_Health.F_AddHealth` _bpc_health (`self.HealAmount`))
    (`KismetSystemLibrary.PrintString` "Use Bandage")
    (set `self.UseItemSuccsee?` true)
    (else
      (set `self.UseItemSuccsee?` false))))

(fn `UserConstructionScript`
  (`parent.UserConstructionScript`))