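; BP_Battery is a usable item that recharges the player's flashlight.
; On UseItem it checks the player's BPCFlashLight component and, if the battery is below maximum, adds BatteryAmount through FAddBatteryLife and prints a debug message.
; It sets the UseItemSuccsee flag to report whether the battery was used, leaving it false when the flashlight is already full.
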(event `self.UseItem`
  (bind _bpc_flashlight (`/Game/Game/Blueprints/BP_Player.BPC_FlashLight` (`self.Player_Ref`)))
  (if (< (`/Game/Game/Blueprints/BlueprintComponent/BPC_FlashLight.CurrentBatteryLevel` _bpc_flashlight) (`/Game/Game/Blueprints/BlueprintComponent/BPC_FlashLight.MaxBatteryLevel` _bpc_flashlight))
    (`/Game/Game/Blueprints/BlueprintComponent/BPC_FlashLight.F_AddBatteryLife` _bpc_flashlight (`self.BatteryAmount`))
    (`KismetSystemLibrary.PrintString` "Use Battery")
    (set `self.UseItemSuccsee?` true)
    (else
      (set `self.UseItemSuccsee?` false))))

(fn `UserConstructionScript`
  (`parent.UserConstructionScript`))