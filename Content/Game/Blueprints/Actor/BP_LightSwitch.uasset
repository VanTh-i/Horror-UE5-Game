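; BP_LightSwitch is an interactable light switch that turns a referenced light on and off.
; Its Interact event checks whether the light component of the Light reference is visible and sets it to the opposite state.
; Each branch also prints a short debug string, and the BeginPlay, overlap and Tick events are unused.
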(event `/Game/Game/Blueprints/Interface/BPI_Interaction.Interact`
  (bind _lightcomponent (`Light.LightComponent` (`self.Light`)))
  (if (`SceneComponent.bVisible` _lightcomponent)
    (`SceneComponent.SetVisibility` _lightcomponent false false)
    (`KismetSystemLibrary.PrintString` "tat")
    (else
      (`SceneComponent.SetVisibility` _lightcomponent true false)
      (`KismetSystemLibrary.PrintString` "bat"))))

(fn `UserConstructionScript`
  (`parent.UserConstructionScript`))