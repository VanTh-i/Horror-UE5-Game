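; BP_Door is an interactable swinging door that toggles open and closed when its Interact event fires.
; On opening, a dot product of the player-to-door direction and the actor's forward vector picks the swing sign, so the side the player stands on decides the direction.
; A timeline lerps the door mesh's yaw between closed and a quarter turn, playing forward to open and in reverse to close.
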(event `self.ReceiveBeginPlay`
  (bind _asbp_player (cast `/Game/Game/Blueprints/BP_Player` (`GameplayStatics.GetPlayerCharacter` 0)))
  (set `self.Player Ref` _asbp_player))

(event `/Game/Game/Blueprints/Interface/BPI_Interaction.Interact`
  (if (`self.IsDoorOpen?`)
    (set `self.IsDoorOpen?` false)
    (bind (_direction _newtrack_0) (`Timeline|Open_Door_Timeline` :!via `ReverseFromEnd` :!label _label)
      (:`Update`
        (`SceneComponent.K2_SetRelativeRotation` (`self.SM_Door`) (`KismetMathLibrary.MakeRotator` 0.0 0.0 (`KismetMathLibrary.Lerp` 0.0 (select `bool` (>= (`self.DotProduct`) 0.0) :`false` -90.0 :`true` 90.0) _newtrack_0)) false false)))
    (else
      (set `self.IsDoorOpen?` true)
      (set `self.DotProduct` (`KismetMathLibrary.Dot_VectorVector` (`KismetMathLibrary.Normal` (- (`self.K2_GetActorLocation` self) (`self.K2_GetActorLocation` (`self.Player Ref`)))) (`self.GetActorForwardVector` self)))
      (goto _label :!via `PlayFromStart`))))

(fn `UserConstructionScript`)