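; Inventory component that holds the player's item slots, sized from the player controller, and refreshes the matching menu grid slot on each change.
; AddItem fills partial stacks, then empty slots, recursing on overflow and returning any remainder.
; UseItem runs the item actor's use logic, spawning one if none exists, and consumes one on success.
; It also drops whole stacks as physics pickups at a camera trace and opens an examination widget.
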(event `self.ReceiveBeginPlay`
  (`self.Initialize`))

(event `Initialize`
  (bind _ashg_player_controller (cast `/Game/Game/Blueprints/HG_PlayerController` (`GameplayStatics.GetPlayerController` 0) :!pure true))
  (`KismetArrayLibrary.Array_Resize` (`self.InventorySlot`) (`/Game/Game/Blueprints/HG_PlayerController.InventorySlot` _ashg_player_controller))
  (set `self.W_InventoryMenu_Ref` (`/Game/Game/Blueprints/HG_PlayerController.W_InventoryMenu_Ref` _ashg_player_controller))
  (bind _asbp_player (cast `/Game/Game/Blueprints/BP_Player` (`GameplayStatics.GetPlayerCharacter` 0)))
  (set `self.Player_Ref` _asbp_player)
  (bind _returnvalue (`|CreateWidget` "/Game/Game/Blueprints/UI/WBP_Examination.WBP_Examination_C" null null))
  (set `self.W_Examination_Ref` _returnvalue)
  (set `/Game/Game/Blueprints/HG_PlayerController.W_Examination_Ref` (`self.W_Examination_Ref`) _ashg_player_controller)
  (bind _outactors (`GameplayStatics.GetAllActorsOfClass` "/Game/Game/Blueprints/Actor/Item/ExaminationItem/BP_Examination.BP_Examination_C"))
  (set `self.BP_Examination_Ref` (`|GetArrayItem` _outactors))
  (set `/Game/Game/Blueprints/UI/WBP_Examination.BPC_Inventory_Ref` self (`self.W_Examination_Ref`)))

(event `CreateExaminationWidget`
  (params (Index :type Integer))
  (bind _w_inventorymenu_ref (`self.W_InventoryMenu_Ref`))
  (`/Game/Game/Blueprints/UI/WBP_Examination.UpdateWidget` (`self.W_Examination_Ref`) Index)
  (`Widget.SetVisibility` _w_inventorymenu_ref "Collapsed")
  (`/Engine/EditorBlueprintResources/StandardMacros.IsValid` (`/Game/Game/Blueprints/UI/WBP_InventoryMenu.WBP_InventoryDropDown` _w_inventorymenu_ref)
    (:`Is Valid`
      (`/Game/Game/Blueprints/UI/WBP_InventoryMenu.CloseDropDownMenu` _w_inventorymenu_ref)
      (`UserWidget.AddToViewport` (`self.W_Examination_Ref`) 2)
      (set `/Game/Game/Blueprints/HG_PlayerController.IsOpenInventory?` false (cast `/Game/Game/Blueprints/HG_PlayerController` (`GameplayStatics.GetPlayerController` 0) :!pure true)))))

(fn `AddItem`
  (params (Item :type "/Game/Game/Blueprints/Actor/Item/BP_ItemMaster Class Reference") (Amount :type Integer))
  (returns (`Success?` :type Boolean) (Remainder :type Integer))
  (locals (LocalItem :type "/Game/Game/Blueprints/Actor/Item/BP_ItemMaster Class Reference") (LocalAmount :type Integer) (LocalMaxStackItem :type Integer) (LocalIndex :type Integer :default 0))
  (bind (_success_ _index) (`self.CheckEmptySlot`))
  (bind (_success__2 _index_2) (`self.CheckEmptySlot`))
  (bind _returnvalue (- (`local.LocalAmount`) 1))
  (bind (_itemname _description _icon _pickupactor _maxstack) (break `/Game/Game/Blueprints/Structs/S_ItemData` (defaults `Object` (`local.LocalItem`))))
  (bind _returnvalue_2 (+ (`.Amount` (`self.GetItemDataAtIndex` (`local.LocalIndex`))) (`local.LocalAmount`)))
  (set `local.LocalItem` Item)
  (set `local.LocalAmount` Amount)
  (set `local.LocalMaxStackItem` _maxstack)
  (if (> _maxstack 1)
    (bind (_success__3 _index_3) (`self.CheckFreeSlot` (`local.LocalItem`)))
    (if _success__3
      (set `local.LocalIndex` _index_3)
      (if (> _returnvalue_2 (`local.LocalMaxStackItem`))
        (set `local.LocalAmount` (- _returnvalue_2 (`local.LocalMaxStackItem`)))
        (`KismetArrayLibrary.Array_Set` (`self.InventorySlot`) (`local.LocalIndex`) (make `/Game/Game/Blueprints/Structs/S_InventoryItem` (`local.LocalItem`) (`local.LocalMaxStackItem`)))
        (`self.UpdateInventorySlot` (`local.LocalIndex`))
        (bind (_success__4 _remainder) (`self.AddItem` (`local.LocalItem`) (`local.LocalAmount`)))
        (return true _remainder)
        (else
          (`KismetArrayLibrary.Array_Set` (`self.InventorySlot`) (`local.LocalIndex`) (make `/Game/Game/Blueprints/Structs/S_InventoryItem` (`local.LocalItem`) _returnvalue_2))
          (`self.UpdateInventorySlot` (`local.LocalIndex`))
          (return true 0)))
      (elif _success_
        (set `local.LocalIndex` _index)
        (if (> (`local.LocalAmount`) (`local.LocalMaxStackItem`))
          (`KismetArrayLibrary.Array_Set` (`self.InventorySlot`) (`local.LocalIndex`) (make `/Game/Game/Blueprints/Structs/S_InventoryItem` (`local.LocalItem`) (`local.LocalMaxStackItem`)))
          (`self.UpdateInventorySlot` (`local.LocalIndex`))
          (bind (_success__5 _remainder_2) (`self.AddItem` (`local.LocalItem`) (- (`local.LocalAmount`) (`local.LocalMaxStackItem`))))
          (return true _remainder_2)
          (else
            (`KismetArrayLibrary.Array_Set` (`self.InventorySlot`) (`local.LocalIndex`) (make `/Game/Game/Blueprints/Structs/S_InventoryItem` (`local.LocalItem`) (`local.LocalAmount`)))
            (`self.UpdateInventorySlot` (`local.LocalIndex`))
            (return true 0)))
        (else
          (return false (`local.LocalAmount`)))))
    (elif _success__2
      (set `local.LocalIndex` _index_2)
      (`KismetArrayLibrary.Array_Set` (`self.InventorySlot`) (`local.LocalIndex`) (make `/Game/Game/Blueprints/Structs/S_InventoryItem` (`local.LocalItem`) 1))
      (`self.UpdateInventorySlot` (`local.LocalIndex`))
      (if (> _returnvalue 0)
        (bind (_success__6 _remainder_3) (`self.AddItem` (`local.LocalItem`) _returnvalue))
        (return true _remainder_3)
        (else
          (return true 0)))
      (else
        (return false (`local.LocalAmount`))))))

(fn `CheckEmptySlot`
  (returns (`Success?` :type Boolean) (Index :type Integer))
  (locals (LocalSuccess :type Boolean) (LocalIndex :type Integer))
  (for (_array_element _array_index) (`self.InventorySlot`)
    (if (`KismetSystemLibrary.IsValidClass` (`.Item_6_8B15EA7B48A58BD55848DFAEF9E448DE` (break `/Game/Game/Blueprints/Structs/S_InventoryItem` _array_element)))
      (set `local.LocalSuccess` false)
      (else
        (set `local.LocalSuccess` true)
        (set `local.LocalIndex` _array_index)
        (break))))
  (return (`local.LocalSuccess`) (`local.LocalIndex`)))

(fn `CheckFreeSlot`
  (params (Item :type "/Game/Game/Blueprints/Actor/Item/BP_ItemMaster Class Reference"))
  (returns (`Success?` :type Boolean) (Index :type Integer))
  (locals (`LocalSuccess?` :type Boolean) (LocalIndex :type Integer))
  (for (_array_element _array_index) (`self.InventorySlot`)
    (bind (_item _amount) (break `/Game/Game/Blueprints/Structs/S_InventoryItem` _array_element))
    (if (and (== _item Item) (< _amount (`.MaxStack_8_B904A030494EBD6A90BF02A6BC55983D` (break `/Game/Game/Blueprints/Structs/S_ItemData` (defaults `Object` Item)))))
      (set `local.LocalSuccess?` true)
      (set `local.LocalIndex` _array_index)
      (break)
      (else
        (set `local.LocalSuccess?` false))))
  (return (`local.LocalSuccess?`) (`local.LocalIndex`)))

(fn `DropItem`
  (params (Index :type Integer))
  (locals (LocalIndex :type Integer) (LocalAmount :type Integer :default 0) (LocalClass :type "/Game/Game/Blueprints/Actor/Item/BP_ItemMaster Class Reference"))
  (bind _camera (`/Game/Game/Blueprints/BP_Player.Camera` (`self.Player_Ref`)))
  (bind _returnvalue (`SceneComponent.K2_GetComponentLocation` _camera))
  (bind _output_get (set `local.LocalIndex` Index))
  (bind (_item _amount) (`self.GetItemDataAtIndex` _output_get))
  (set `local.LocalAmount` _amount)
  (set `local.LocalClass` _item)
  (if (> (`local.LocalAmount`) 0)
    (for _ (range (`local.LocalAmount`))
      (`self.RemoveItemUse` (`local.LocalIndex`)))
    (`/Game/Game/Blueprints/UI/WBP_InventoryMenu.CloseDropDownMenu` (`self.W_InventoryMenu_Ref`))
    (bind (_outhit _returnvalue_2) (`KismetSystemLibrary.LineTraceSingle` _returnvalue (+ _returnvalue (* (`SceneComponent.GetForwardVector` _camera) 200.0)) "TraceTypeQuery1"))
    (bind (_bblockinghit _binitialoverlap _time _distance _location _impactpoint _normal _impactnormal _physmat _hitactor _hitcomponent _hitbonename _bonename _hititem _elementindex _faceindex _tracestart _traceend) (`GameplayStatics.BreakHitResult` _outhit))
    (bind _returnvalue_3 (`|SpawnActorFromClass` (`.PickUpActor_16_D7C1806748CCEE0EF7D9DF8772811F30` (break `/Game/Game/Blueprints/Structs/S_ItemData` (defaults `Object` (`local.LocalClass`)))) (`KismetMathLibrary.MakeTransform` (select `bool` _returnvalue_2 :`false` _traceend :`true` _location)) "Undefined" "MultiplyWithRoot" null null))
    (set `/Game/Game/Blueprints/Actor/Item/BP_PickupMaster.Amount` (`local.LocalAmount`) _returnvalue_3)
    (`PrimitiveComponent.SetSimulatePhysics` (`/Game/Game/Blueprints/Actor/Item/BP_PickupMaster.StaticMesh` _returnvalue_3) true)))

(fn `GetItemDataAtIndex`
  (params (Index :type Integer))
  (returns (Item :type "/Game/Game/Blueprints/Actor/Item/BP_ItemMaster Class Reference") (Amount :type Integer))
  (bind (_item _amount) (break `/Game/Game/Blueprints/Structs/S_InventoryItem` (`|GetArrayItem` (`self.InventorySlot`) Index)))
  (return _item _amount))

(fn `RemoveItemUse`
  (params (Index :type Integer))
  (bind (_item _amount) (`self.GetItemDataAtIndex` Index))
  (if (> _amount 1)
    (`KismetArrayLibrary.Array_Set` (`self.InventorySlot`) Index (make `/Game/Game/Blueprints/Structs/S_InventoryItem` _item (- _amount 1)))
    (else
      (`KismetArrayLibrary.Array_Set` (`self.InventorySlot`) Index (make `/Game/Game/Blueprints/Structs/S_InventoryItem` null))))
  (`self.UpdateInventorySlot` Index))

(fn `UpdateInventorySlot`
  (params (Index :type Integer))
  (`/Game/Game/Blueprints/UI/WBP_InventorySlot.F_UpdateSlot` (`|GetArrayItem` (`/Game/Game/Blueprints/UI/WBP_InventoryGrid.SlotArray` (`/Game/Game/Blueprints/UI/WBP_InventoryMenu.WBP_InventoryGrid` (`/Game/Game/Blueprints/HG_PlayerController.W_InventoryMenu_Ref` (cast `/Game/Game/Blueprints/HG_PlayerController` (`GameplayStatics.GetPlayerController` 0) :!pure true)))) Index)))

(fn `UseItem`
  (params (Index :type Integer))
  (locals (LocalIndex :type Integer))
  (bind (_item _amount) (`self.GetItemDataAtIndex` Index))
  (set `local.LocalIndex` Index)
  (if (> _amount 0)
    (bind _returnvalue (`GameplayStatics.GetActorOfClass` _item))
    (`/Engine/EditorBlueprintResources/StandardMacros.IsValid` _returnvalue
      (:`Is Valid`
        (`/Game/Game/Blueprints/Actor/Item/BP_ItemMaster.UseItem` _returnvalue)
        (if (`/Game/Game/Blueprints/Actor/Item/BP_ItemMaster.UseItemSuccsee?` _returnvalue)
          (`self.RemoveItemUse` (`local.LocalIndex`) :!label _label)
          (`/Game/Game/Blueprints/UI/WBP_InventoryMenu.CloseDropDownMenu` (`self.W_InventoryMenu_Ref`))))
      (:`Is Not Valid`
        (bind _returnvalue_2 (`|SpawnActorFromClass` _item (`KismetMathLibrary.MakeTransform` (0.0 0.0 0.0)) "Undefined" "MultiplyWithRoot" null null))
        (`/Game/Game/Blueprints/Actor/Item/BP_ItemMaster.UseItem` _returnvalue_2)
        (if (`/Game/Game/Blueprints/Actor/Item/BP_ItemMaster.UseItemSuccsee?` _returnvalue_2)
          (goto _label))))))