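; Flashlight component that toggles the player's light and manages its battery life.
; Initialize caches the player and its FlashLight, and toggling on requires charge above the minimum and starts a looping depletion timer.
; Each drain tick or battery pickup amount clamps the level and remaps it to the light's IES brightness scale, dimming only at low charge.
; An empty battery hides the light and clears the timer.
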(fn `F_AddBatteryLife`
  (params (Amount :type "Float (double-precision)"))
  (set `self.CurrentBatteryLevel` (`KismetMathLibrary.FClamp` (+ (`self.CurrentBatteryLevel`) Amount) (`self.MinBatteryLevel`) (`self.MaxBatteryLevel`)))
  (`self.F_SetIntensity`))

(fn `F_DepleteBatteryLife`
  (bind _output_get (set `self.CurrentBatteryLevel` (`KismetMathLibrary.FClamp` (- (`self.CurrentBatteryLevel`) (`self.DepletionAmount`)) (`self.MinBatteryLevel`) (`self.MaxBatteryLevel`))))
  (`self.F_SetIntensity`)
  (if (<= _output_get (`self.MinBatteryLevel`))
    (`SceneComponent.SetVisibility` (`self.Light`) false false)
    (`KismetSystemLibrary.K2_ClearTimer` null "F_DepleteBatteryLife")))

(fn `F_SetIntensity`
  (`LightComponent.SetIESBrightnessScale` (`self.Light`) (`KismetMathLibrary.MapRangeClamped` (`self.CurrentBatteryLevel`) (`self.MinBatteryLevel`) 20.0 0.0 1.0)))

(fn `F_ToggleFlashLight`
  (bind _light (`self.Light`))
  (if (`SceneComponent.bVisible` _light)
    (`SceneComponent.SetVisibility` _light false false)
    (`KismetSystemLibrary.K2_ClearTimer` null "F_DepleteBatteryLife")
    (elif (> (`self.CurrentBatteryLevel`) (`self.MinBatteryLevel`))
      (`self.F_SetIntensity`)
      (`SceneComponent.SetVisibility` _light true false)
      (`KismetSystemLibrary.K2_SetTimer` null "F_DepleteBatteryLife" (`self.DepletionSpeed`) true))))

(fn `Initialize`
  (params (Player :type "/Game/Game/Blueprints/BP_Player Object Reference"))
  (bind _output_get (set `self.Player_Ref` Player))
  (set `self.Light` (`/Game/Game/Blueprints/BP_Player.FlashLight` _output_get)))