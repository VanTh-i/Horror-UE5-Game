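; BPC_Health is a health component that tracks current health and drives a blood screen effect from it.
; Functions to remove or add health clamp the value between minimum and maximum, then refresh the effect, which also refreshes on BeginPlay.
; The refresh writes a scalar to the MPC_BloodScreen parameter collection, rising from half to full as health climbs to about 70% of its range, then holding.
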(event `self.ReceiveBeginPlay`
  (`self.F_UpdateBloodScreen`))

(fn `F_AddHealth`
  (params (Amount :type "Float (double-precision)"))
  (set `self.CurrentHealth` (`KismetMathLibrary.FClamp` (+ (`self.CurrentHealth`) Amount) (`self.MinHealth`) (`self.MaxHealth`)))
  (`self.F_UpdateBloodScreen`))

(fn `F_RemoveHealth`
  (params (Amount :type "Float (double-precision)"))
  (set `self.CurrentHealth` (`KismetMathLibrary.FClamp` (- (`self.CurrentHealth`) Amount) (`self.MinHealth`) (`self.MaxHealth`)))
  (`self.F_UpdateBloodScreen`))

(fn `F_UpdateBloodScreen`
  (`KismetMaterialLibrary.SetScalarParameterValue` "/Game/Game/Material/MPC_BloodScreen.MPC_BloodScreen" "Amount" (`KismetMathLibrary.MapRangeClamped` (`self.CurrentHealth`) (`self.MinHealth`) (* (- (`self.MaxHealth`) (`self.MinHealth`)) 0.7) 0.5 1.0)))